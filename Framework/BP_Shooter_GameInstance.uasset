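; Game instance for a shooter that owns the main menu and starts solo games.
; UIShowMainMenu creates the main menu widget if no valid one is cached, adds it to the viewport, and switches the first player controller to UI-only input with a visible cursor.
; Start_SoloGame sets the IsSoloGame flag on the instance, then opens Map0 by name.
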(event `Start_SoloGame`
  (set `self.IsSoloGame` true)
  (`GameplayStatics.OpenLevel` "Map0"))

(fn `UI_ShowMainMenu`
  (bind _returnvalue (`GameplayStatics.GetPlayerController` 0))
  (`/Engine/EditorBlueprintResources/StandardMacros.IsValid` (`self.MainMenu`)
    (:`Is Valid`
      _)
    (:`Is Not Valid`
      (bind _returnvalue_2 (`|CreateWidget` "/Game/Widgets/WBP_MainMenu.WBP_MainMenu_C" _returnvalue))
      (set `self.MainMenu` _returnvalue_2)))
  (`UserWidget.AddToViewport` (`self.MainMenu`) 0)
  (`WidgetBlueprintLibrary.SetInputMode_UIOnlyEx` _returnvalue null)
  (set `PlayerController.bShowMouseCursor` true _returnvalue)
  (return))